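; Test game mode that gives joining players a persistent ID and hosts the trade manager for the multiplayer inventory system.
; PostLogin keeps an ID already in its list, otherwise writes a new GUID string to the MP_Inventory_PlayerState, records it and prints it.
; BeginPlay constructs BP_Trading_Manager.
; Item definition storage creation and sample trade calls are left unconnected, so never run.
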(event `self.K2_PostLogin`
  (params (NewPlayer :type "PlayerController Object Reference"))
  (bind _persistent_player_list (`self.Persistent Player List`))
  (bind _returnvalue (`KismetGuidLibrary.Conv_GuidToString` (`KismetGuidLibrary.NewGuid`)))
  ; Set Uniqueid For MP_Inventory_PlayerState
  (bind _asmp_inventory_player_state (cast `MP_Inventory_PlayerState` (`Controller.PlayerState` NewPlayer)))
  (bind _persistentplayerid (`MP_Inventory_PlayerState.PersistentPlayerId` _asmp_inventory_player_state))
  (if (not (`BlueprintSetLibrary.Set_Contains` _persistent_player_list _persistentplayerid))
    (if (`BlueprintSetLibrary.Set_Contains` _persistent_player_list _returnvalue) :!label _label
      (`KismetSystemLibrary.Delay` 0.2)
      (goto _label)
      (else
        (bind _output_get (set `MP_Inventory_PlayerState.PersistentPlayerId` _returnvalue _asmp_inventory_player_state))
        (`BlueprintSetLibrary.Set_Add` _persistent_player_list _output_get))))
  (`KismetSystemLibrary.PrintString` _persistentplayerid true true (struct :`R` 0.145044 :`G` 1.0 :`A` 1.0)))

(event `self.ReceiveBeginPlay`
  ; Initlization
  (bind _returnvalue (`|GenericCreateObject` "/MP_Inventory/Utility/BP_Trading_Manager.BP_Trading_Manager_C"))
  (set `self.Trade Manager` _returnvalue))

(fn `UserConstructionScript`)